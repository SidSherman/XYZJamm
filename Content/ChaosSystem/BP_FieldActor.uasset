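; BP_FieldActor is a Chaos field actor that applies external cluster strain, used to break Geometry Collections within a sphere.
; Toggle and CallTriggerActor events share one path: a short delay, then a radial falloff field applied through the FieldSystemComponent.
; The Trigger sphere supplies center and radius, Magnitude sets strength, and falloff is none.
; A parameterless Toggle calls EventToggle with false; the Onoff input goes unused.
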(event Custom|Toggle
  (CallFunction|EventToggle false))

(event Custom|Event%20Toggle
  (params (On/off :type Boolean))
  (bind _trigger (Variables|Default|GetTrigger))
  (Utilities|FlowControl|Delay 0.2)
  (Class|FieldSystemComponent|ApplyPhysicsField (Variables|Field|GetFieldSystemComponent) true "Field_ExternalClusterStrain" 0 (Field|SetRadialFalloff (Variables|Default|GetRadialFalloff) (Variables|Default|GetMagnitude) 0.0 1.0 0.0 (Components|Sphere|GetScaledSphereRadius _trigger) (Transformation|GetWorldLocation _trigger) "Field_FallOff_None")))

(event Custom|Event%20Call%20Trigger%20Actor
  (bind _trigger (Variables|Default|GetTrigger))
  (Utilities|FlowControl|Delay 0.2)
  (Class|FieldSystemComponent|ApplyPhysicsField (Variables|Field|GetFieldSystemComponent) true "Field_ExternalClusterStrain" 0 (Field|SetRadialFalloff (Variables|Default|GetRadialFalloff) (Variables|Default|GetMagnitude) 0.0 1.0 0.0 (Components|Sphere|GetScaledSphereRadius _trigger) (Transformation|GetWorldLocation _trigger) "Field_FallOff_None")))

(event EventTick
  (params (DeltaSeconds :type Float%20%28single-precision%29)))

(event EventBeginPlay)

(event Collision|EventActorBeginOverlap
  (params (OtherActor :type Actor%20Object%20Reference)))

(fn ConstructionScript)