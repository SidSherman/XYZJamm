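; Chaos field system actor that applies a disable threshold to physics bodies within a box, despite its SleepField name.
; Every Tick builds a box falloff carrying the Threshold value and wraps it in a culling field that culls outside the Trigger's box.
; The result goes to the FieldSystemComponent as a disable-threshold physics field, using the Trigger's current world transform each frame.
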(event EventBeginPlay)

(event Collision|EventActorBeginOverlap
  (params (OtherActor :type Actor%20Object%20Reference)))

(event EventTick
  (params (DeltaSeconds :type Float%20%28single-precision%29))
  (bind _trigger (Variables|Default|GetTrigger))
  (bind _returnvalue (Transformation|GetWorldTransform _trigger))
  (Class|FieldSystemComponent|ApplyPhysicsField (Variables|Field|GetFieldSystemComponent) true "Field_DisableThreshold" 0 (Field|SetCullingField (Variables|Default|GetCullingField) (Field|SetBoxFalloff (Variables|Default|GetBoxFalloff%20-%20Culling) 1.0 0.0 1.0 0.0 _returnvalue "Field_FallOff_None") (Field|SetBoxFalloff (Variables|Default|GetBoxFalloff) (Variables|Default|GetThreshold) 1.0 1.0 0.0 _returnvalue "Field_FallOff_None") "Field_Culling_Outside")))

(fn ConstructionScript)