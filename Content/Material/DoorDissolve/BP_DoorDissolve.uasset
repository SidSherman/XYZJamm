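; BP_DoorDissolve is an interactive door that dissolves open and re-forms when E is pressed.
; A trigger overlap enables input and shows two text prompts.
; E toggles Closed, driving the TimeDissolve timeline forward or backward to animate the door material's Radius parameter, with sound and delayed collision changes.
; Timeline updates also rewrite Closed from progress, so true corresponds to the dissolved state despite its name.
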(event OnComponentBeginOverlap(Trigger)
  (params (OverlappedComponent :type Primitive%20Component%20Object%20Reference) (OtherActor :type Actor%20Object%20Reference) (OtherComp :type Primitive%20Component%20Object%20Reference) (OtherBodyIndex :type Integer) (bFromSweep :type Boolean) (SweepResult :type Hit%20Result%20Structure%20%28by%20ref%29))
  (Input|EnableInput (Game|GetPlayerController 0))
  (Rendering|SetVisibility (Variables|Default|GetTextOpen1) true false))

(event OnComponentEndOverlap(Trigger)
  (params (OverlappedComponent :type Primitive%20Component%20Object%20Reference) (OtherActor :type Actor%20Object%20Reference) (OtherComp :type Primitive%20Component%20Object%20Reference) (OtherBodyIndex :type Integer))
  (Input|DisableInput (Game|GetPlayerController 0))
  (Rendering|SetVisibility (Variables|Default|GetTextOpen1) false false))

(event EventBeginPlay)

(event Collision|EventActorBeginOverlap
  (params (OtherActor :type Actor%20Object%20Reference)))

(event EventTick
  (params (DeltaSeconds :type Float%20%28single-precision%29)))

(event Input|KeyboardEvents|E
  (params (Key :type Key%20Structure :default "None"))
  (:Pressed
    (bind _output_get (Variables|Default|SetClosed (not (Variables|Default|GetClosed))))
    (if _output_get
      (Audio|SpawnSound2D "/Game/Sound/DoorDissolve.DoorDissolve" 1.0 1.0 0.0 0)
      (Utilities|FlowControl|Sequence
        (:then_0
          (Utilities|FlowControl|Delay 1.0)
          (Collision|SetCollisionEnabled (Variables|Default|GetDoor) "NoCollision")
          (Rendering|SetVisibility (Variables|Default|GetTextOpen1) false false))
        (:then_1
          (bind _line (Timeline|TimeDissolve Play)
            (:Update
              (Rendering|Material|SetScalarParameterValueonMaterials (Variables|Default|GetDoor) "Radius" (Math|Float|Lerp 0.0 0.7 _line))
              (Variables|Default|SetClosed (> _line 0.9))))))
      (else
        (Utilities|FlowControl|Delay 0.7)
        (Audio|SpawnSound2D "/Game/Sound/DoorDissolve.DoorDissolve" 1.0 1.0 0.0 0)
        (Utilities|FlowControl|Sequence
          (:then_0
            (Timeline|TimeDissolve Reverse))
          (:then_1
            (Collision|SetCollisionEnabled (Variables|Default|GetDoor) "QueryAndPhysics")))))))

(fn ConstructionScript)