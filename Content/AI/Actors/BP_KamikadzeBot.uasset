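; Kamikaze AI bot that damages the player character on mesh overlap and then destroys itself.
; While it has a valid target, each tick runs a forward sphere trace from below the mesh, ignoring itself and the target.
; A hit nudges the mesh upward to clear the obstacle, otherwise its height eases toward the target's.
; This file adjusts only height, with swept moves, and also calls the parent's BeginPlay and Tick.
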(event OnComponentBeginOverlap(Mesh)
  (params (OverlappedComponent :type Primitive%20Component%20Object%20Reference) (OtherActor :type Actor%20Object%20Reference) (OtherComp :type Primitive%20Component%20Object%20Reference) (OtherBodyIndex :type Integer) (bFromSweep :type Boolean) (SweepResult :type Hit%20Result%20Structure%20%28by%20ref%29))
  (Development|PrintString "Hello")
  (bind _asbp_player_character (Utilities|Casting|CastToBP_PlayerCharacter OtherActor))
  (Game|Damage|ApplyDamage _asbp_player_character (Variables|Default|GetBase%20Damage) 0 0)
  (Actor|DestroyActor))

(event EventBeginPlay
  (|CallParentFunction))

(event EventTick
  (params (DeltaSeconds :type Float%20%28single-precision%29))
  (bind _mesh (Variables|Character|GetMesh))
  (bind _mesh_2 (Variables|Character|GetMesh))
  (bind _returnvalue (Transformation|GetWorldLocation _mesh))
  (bind _returnvalue_2 (Transformation|GetWorldLocation _mesh_2))
  (bind (_x _y _z) (Math|Vector|BreakVector _returnvalue_2))
  (bind (_x_2 _y_2) (Math|Vector|BreakVector _returnvalue))
  (bind _returnvalue_3 (- _returnvalue "0,0,45.000000"))
  (|CallParentFunction DeltaSeconds)
  (bind _targetactor (Variables|Default|GetTargetActor)
    (:then
      (bind _returnvalue_4 (Collision|SphereTraceByChannel _returnvalue_3 (+ _returnvalue_3 (* (Math|Vector|GetForwardVector _mesh) 1e+02)) 1e+01 "TraceTypeQuery1" false (Utilities|Array|MakeArray _targetactor self) "ForOneFrame"))
      (if _returnvalue_4
        (Transformation|SetWorldLocation _mesh_2 (Math|Interpolation|VInterpTo _returnvalue_2 (Math|Vector|MakeVector _x _y (+ _z 5.0)) DeltaSeconds 5e+01) true false)
        (else
          (Transformation|SetWorldLocation (Variables|Character|GetMesh) (Math|Interpolation|VInterpTo _returnvalue (Math|Vector|MakeVector _x_2 _y_2 (.Z (Math|Vector|BreakVector (Transformation|GetActorLocation _targetactor)))) DeltaSeconds 1.0) true false))))
    (:else)))

(fn ConstructionScript)