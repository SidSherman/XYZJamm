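; Boss character for the ranged AI, dual-wielding two spawned weapons and driven by a Blackboard.
; On BeginPlay it caches its ranged AI controller, attaches a weapon to each hand socket and writes the EQS flag to the Blackboard.
; It starts in one AI state and switches to another after a short delay.
; On death it runs the parent logic, then after a delay enables mesh physics with a very low blend weight.
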(event EventBeginPlay
  (bind _returnvalue (AI|GetBlackboard 0))
  (bind _self self)
  (bind _self_2 self)
  ;[1 1 1] begin Play
  (Utilities|IsValid _returnvalue
    (:Is%20Valid
      (bind _output_get (Variables|Default|SetAIState "NewEnumerator3"))
      (AI|Components|Blackboard|SetValueasEnum _returnvalue (Variables|Default|GetAIStateBBKey) _output_get)
      (Utilities|FlowControl|Sequence
        (:then_0
          (bind _asaic_ranged_ai (Utilities|Casting|CastToAIC_RangedAI (Pawn|GetController)))
          (Variables|Default|SetAIController _asaic_ranged_ai))
        (:then_1
          (bind _returnvalue_2 (Game|SpawnActorfromClass (Variables|Default|GetWeaponClass) (Transformation|GetActorTransform) "AlwaysSpawn" _self_2 _self_2))
          (Transformation|AttachComponentToComponent _returnvalue_2 (Variables|Character|GetMesh) "RightWeaponSocket" "SnapToTarget" "SnapToTarget" "KeepRelative" true)
          (Variables|Default|SetRightWeapon _returnvalue_2)
          (bind _returnvalue_3 (Game|SpawnActorfromClass (Variables|Default|GetWeaponClass) (Transformation|GetActorTransform) "AlwaysSpawn" _self _self))
          (Transformation|AttachComponentToComponent _returnvalue_3 (Variables|Character|GetMesh) "LeftWeaponSocket" "SnapToTarget" "SnapToTarget" "KeepRelative" true)
          (Variables|Default|SetLeftWeapon _returnvalue_3))
        (:then_2
          (AI|Components|Blackboard|SetValueasBool (AI|GetBlackboard 0) (Variables|Default|GetShouldUseEQSBBKey) (Variables|Default|GetbShouldUseEQS)))
        (:then_3
          (Utilities|FlowControl|Delay 5.0)
          (bind _output_get_2 (Variables|Default|SetAIState "NewEnumerator0"))
          (AI|Components|Blackboard|SetValueasEnum (AI|GetBlackboard 0) (Variables|Default|GetAIStateBBKey) _output_get_2))))))

(event Collision|EventActorBeginOverlap
  (params (OtherActor :type Actor%20Object%20Reference))
  (|CallParentFunction OtherActor) ; This node is disabled and will not be called.\nDrag off pins to build functionality.
)

(event EventTick
  (params (DeltaSeconds :type Float%20%28single-precision%29))
  (|CallParentFunction DeltaSeconds) ; This node is disabled and will not be called.\nDrag off pins to build functionality.
)

(event EventOnDeathEvent
  (bind _mesh (Variables|Character|GetMesh))
  ;[1 1 1] On Death
  (|CallParentFunction)
  (Utilities|FlowControl|Delay 1.2)
  (Physics|SetSimulatePhysics _mesh true)
  (Class|SkeletalMeshComponent|SetPhysicsBlendWeight _mesh 0.01))

(fn ConstructionScript
  (|CallParentFunction))