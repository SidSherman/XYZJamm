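; Base AI character that drives blackboard alert and combat states from sight and hearing of the player.
; Sighting makes noise at the player and turns aggressive on a timer or proximity; a timer handles losing sight.
; Tick traces below the target to update its blackboard position; noises set that position while no target exists.
; It also seeds patrol points, plays random melee and damage-scaled hit montages, and deactivates and unpossesses on death.
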(event OnPerceptionUpdated(AIPerception)
  (params (UpdatedActors :type Array%20of%20Actor%20Object%20References))
  (bind _out (CallFunction|GetCharfrom UpdatedActors))
  (bind _returnvalue (AI|GetBlackboard 0))
  ;[0.1521 0.477 1] Sight Reciver
  ;;[1 1 1] FindPlayerCharacter
  (Utilities|IsValid (AI|GetBlackboard 0)
    (:Is%20Valid
      (Utilities|IsValid _out
        (:Is%20Valid
          (if (!= (Utilities|Array|FindItem (Class|AIPerceptionComponent|GetCurrentlyPerceivedActors (Variables|Default|GetAIPerception) "/Script/AIModule.AISense_Sight") _out) -1)
            (bind _output_get (Variables|AIBehaviour|SetTargetActor _out))
            (Utilities|Time|ClearandInvalidateTimerbyHandle (Variables|AIBehaviour|GetSightForgetHandle))
            ;;[1 1 1] Make Noise at Target Actor
            (Utilities|IsValid (AI|Components|Blackboard|GetValueasObject (AI|GetBlackboard 0) (Variables|AIBehaviour|Blackboard|GetTargetActorBBKey))
              (:Is%20Valid
                _)
              (:Is%20Not%20Valid
                (bind _aspawn (Utilities|Casting|CastToPawn (Variables|AIBehaviour|GetTargetActor))
                  (:then
                    (Class|Actor|MakeNoise _output_get 1e+03 _aspawn (Transformation|GetActorLocation (Variables|AIBehaviour|GetTargetActor)) 3e+03 "Noise"))
                  (:CastFailed
                    _))))
            ;;[1 1 1] Set Target
            (Utilities|IsValid _returnvalue
              (:Is%20Valid
                (AI|Components|Blackboard|SetValueasObject _returnvalue (Variables|AIBehaviour|Blackboard|GetTargetActorBBKey) (Variables|AIBehaviour|GetTargetActor))
                (AI|Components|Blackboard|SetValueasBool _returnvalue (Variables|AIBehaviour|Blackboard|GetHasLostTimerBBKey) false)
                ;;;[1 1 1] Time To SetArressiveState
                (bind _returnvalue_2 (Utilities|Time|SetTimerbyEvent (delegate Custom|CatiousTimer) (Variables|AIBehaviour|GetCatiousTime)))
                (Variables|AIBehaviour|SetCatiousTimerHandle _returnvalue_2)
                (Utilities|IsValid (Variables|AIBehaviour|GetTargetActor)
                  (:Is%20Valid
                    (if (<= (Math|Vector|Distance(Vector) (Transformation|GetActorLocation (Variables|AIBehaviour|GetTargetActor)) (Transformation|GetActorLocation)) (Variables|Combat|GetAgressiveDistance))
                      (CallFunction|CatiousTimer))))))
            (else
              (bind _returnvalue_3 (Utilities|Time|SetTimerbyEvent (delegate Custom|SightForgetEvent) (Variables|AIBehaviour|GetTimeToForgetPlayer)))
              (Variables|AIBehaviour|SetSightForgetHandle _returnvalue_3))))))))

(event OnTargetPerceptionUpdated(AIPerception)
  (params (Actor :type Actor%20Object%20Reference) (Stimulus :type AI%20Stimulus%20Structure))
  ;[1 0.8899 0.1083] Hearing Reciever
  (Utilities|IsValid (AI|GetBlackboard 0)
    (:Is%20Valid
      (if (== (.tag Stimulus) "Noise")
        (Utilities|IsValid (AI|Components|Blackboard|GetValueasObject (AI|GetBlackboard 0) (Variables|AIBehaviour|Blackboard|GetTargetActorBBKey))
          (:Is%20Not%20Valid
            (Utilities|Casting|CastToBP_PlayerCharacter Actor)
            (Development|PrintString "AI Heard Player" true true "(R=0.000000,G=0.660000,B=1.000000,A=1.000000)" 2.0 "2")
            (AI|Components|Blackboard|SetValueasBool (AI|GetBlackboard 0) (Variables|AIBehaviour|Blackboard|GetTargetPositionUpdatedBBKey) true)
            (switch Utilities|FlowControl|Switch|SwitchonEAIStates (Variables|AIBehaviour|GetAIState)
              (:NewEnumerator0
                (bind _output_get (Variables|AIBehaviour|SetAIState "NewEnumerator1"))
                (AI|Components|Blackboard|SetValueasEnum (AI|GetBlackboard 0) (Variables|AIBehaviour|Blackboard|GetAIStateBBKey) _output_get))
              (:NewEnumerator1
                _)
              (:NewEnumerator2
                _)
              (:NewEnumerator4
                _))
            (AI|Components|Blackboard|SetValueasVector (AI|GetBlackboard 0) (Variables|AIBehaviour|Blackboard|GetTargetPositionBBKey) (.stimuluslocation Stimulus))
            (AI|Components|Blackboard|SetValueasBool (AI|GetBlackboard 0) (Variables|AIBehaviour|Blackboard|GetHeardSometingBBKey) true)))))))

(event Custom|CustomEvent
  (params (UpdatedActors :type Array%20of%20Actor%20Object%20References))
  ;[1 1 1] Debug
)

(event Custom|CatiousTimer
  ;[0.1521 0.477 1] Sight Reciver
  ;;[1 1 1] Set Target
  ;;;[1 1 1] Time To SetArressiveState
  (AI|Components|Blackboard|ClearValue (AI|GetBlackboard 0) (Variables|AIBehaviour|Blackboard|GetHasLostTimerBBKey))
  (Utilities|Time|ClearandInvalidateTimerbyHandle (Variables|AIBehaviour|GetCatiousTimerHandle))
  (bind _output_get (Variables|AIBehaviour|SetAIState "NewEnumerator2"))
  (AI|Components|Blackboard|SetValueasEnum (AI|GetBlackboard 0) (Variables|AIBehaviour|Blackboard|GetAIStateBBKey) _output_get))

(event Custom|SightForgetEvent
  (bind _returnvalue (AI|GetBlackboard 0))
  ;[0.1521 0.477 1] Sight Reciver
  ;;[1 1 1] Forget About Target
  (Utilities|Time|ClearandInvalidateTimerbyHandle (Variables|AIBehaviour|GetSightForgetHandle))
  (if (Utilities|Enum|Equal(Enum) (Variables|AIBehaviour|GetAIState) "NewEnumerator0")
    (bind _output_get (Variables|AIBehaviour|SetAIState "NewEnumerator1"))
    (Utilities|IsValid _returnvalue
      (:Is%20Valid
        (AI|Components|Blackboard|SetValueasEnum _returnvalue (Variables|AIBehaviour|Blackboard|GetAIStateBBKey) _output_get))))
  (AI|Components|Blackboard|SetValueasBool (AI|GetBlackboard 0) (Variables|AIBehaviour|Blackboard|GetHasLostTimerBBKey) true)
  (bind _targetactor (Utilities|GetTargetPosotion)
    (:HitResultIsValid
      (AI|Components|Blackboard|ClearValue _targetactor (Variables|AIBehaviour|Blackboard|GetTargetActorBBKey) :!label _label))
    (:HitResultIsntValid
      (if (Utilities|Enum|Equal(Enum) (Variables|AIBehaviour|GetAIState) "NewEnumerator2")
        (Variables|AIBehaviour|SetAIState "NewEnumerator4")
        (goto _label)))))

(event Custom|PlayMeleeAttackMontage
  ;[1 1 1] MeleeAttack
  (bind _output_get (Variables|Combat|SetCombatState "NewEnumerator5"))
  (AI|Components|Blackboard|SetValueasEnum (AI|GetBlackboard 0) (Variables|AIBehaviour|Blackboard|GetCombatStateBBKey) _output_get)
  (Animation|Montage|PlayMontage (Variables|Character|GetMesh) (.OutItem (Utilities|Array|Random (Variables|Combat|GetMeleeMontages)))
    (:OnCompleted
      (bind _output_get_2 (Variables|Combat|SetCombatState "NewEnumerator2"))
      (AI|Components|Blackboard|SetValueasEnum (AI|GetBlackboard 0) (Variables|AIBehaviour|Blackboard|GetCombatStateBBKey) _output_get_2))))

(event Custom|StartMeleeAttack
  ;[1 1 1] MeleeAttack
)

(event Custom|EndMeleeAttack
  ;[1 1 1] MeleeAttack
)

(event Game|Damage|EventAnyDamage
  (params (Damage :type Float%20%28single-precision%29) (DamageType :type Damage%20Type%20Object%20Reference) (InstigatedBy :type Controller%20Object%20Reference) (DamageCauser :type Actor%20Object%20Reference))
  (bind _weakdamage (Variables|Default|GetWeakDamage))
  (bind _weakhitmontages (Variables|Combat|GetWeakHitMontages))
  (bind _stronghitmontages (Variables|Combat|GetStrongHitMontages))
  (bind _returnvalue (<= Damage _weakdamage))
  (bind _returnvalue_2 (select _returnvalue _weakhitmontages _stronghitmontages))
  ;[1 1 1] Get Damage
  (Utilities|IsValid (AI|GetBlackboard 0)
    (:Is%20Valid
      (if (Utilities|Enum|NotEqual(Enum) (Variables|AIBehaviour|GetAIState) "NewEnumerator3")
        (if (Utilities|Array|IsNotEmpty _returnvalue_2)
          (if _returnvalue
            _
            (else
              (Variables|Combat|SetCombatState "NewEnumerator6")))
          (Animation|Montage|PlayMontage (Variables|Character|GetMesh) (.OutItem (Utilities|Array|Random _returnvalue_2))
            (:OnCompleted
              (Variables|Combat|SetCombatState "NewEnumerator2"))))
        (bind _output_get (Variables|Default|SetCurrentHealth (- (Variables|Default|GetCurrentHealth) Damage)))
        (if (<= _output_get 0.0)
          (CallFunction|OnDeathEvent))))))

(event EventTick
  (params (DeltaSeconds :type Float%20%28single-precision%29))
  ;[1 1 1] Debug
  (Utilities|IsValid (AI|GetBlackboard 0)
    (:Is%20Valid
      (Utilities|GetTargetPosotion))))

(event EventOnDeathEvent
  ;[1 1 1] On Death
  (|CallParentFunction)
  (Utilities|IsValid (AI|GetBlackboard 0)
    (:Is%20Valid
      (bind _output_get (Variables|AIBehaviour|SetAIState "NewEnumerator3"))
      (AI|Components|Blackboard|SetValueasEnum (AI|GetBlackboard 0) (Variables|AIBehaviour|Blackboard|GetAIStateBBKey) _output_get)
      (Collision|SetCollisionEnabled (Variables|Default|GetCapsuleComponent) "NoCollision")
      (Pawn|UnPossess (AI|GetAIController self)))))

(event EventBeginPlay
  ;[1 1 1] Set patrollin point
  (|CallParentFunction)
  (Utilities|IsValid (AI|GetBlackboard 0)
    (:Is%20Valid
      (if (Utilities|Array|IsNotEmpty (Variables|Patrolling|GetPatrollingPoints))
        (Variables|Patrolling|SetCurrentPatrollingPoint (Utilities|Array|Get(acopy) (Variables|Patrolling|GetPatrollingPoints)))
        (Variables|Patrolling|SetCurrentPatrollingPointIndex -1))
      (AI|Components|Blackboard|SetValueasEnum (AI|GetBlackboard 0) (Variables|AIBehaviour|Blackboard|GetCombatStateBBKey) (Variables|Combat|GetCombatState)))))

(fn ConstructionScript
  (|CallParentFunction))

(fn GetCharfrom
  (params (Input :type Array%20of%20Actor%20Object%20References))
  (for _array_element Input
    (bind _asbp_player_character (Utilities|Casting|CastToBP_PlayerCharacter _array_element))
    (return _asbp_player_character)))