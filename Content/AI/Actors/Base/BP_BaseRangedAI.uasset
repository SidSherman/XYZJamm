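; Base Blueprint for ranged AI characters, handling aiming, shooting and weapon cleanup on death.
; On BeginPlay it caches its AIC_RangedAI controller and writes the ShouldUseEQS setting to the blackboard.
; Starting or stopping aim updates IsAiming and the CombatState enum, mirrored to the blackboard.
; Attacks loop by replaying the shoot montage on completion until StopAttack stops it, and death destroys both weapon actors.
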(event Custom|StopAttack
  ;[1 1 1] Shooting
  (Animation|StopAnimMontage (Variables|Combat|GetShootMontages)))

(event Custom|Attack
  ;[1 1 1] Shooting
  (Animation|Montage|PlayMontage (Variables|Character|GetMesh) (Variables|Combat|GetShootMontages)
    (:OnCompleted
      (CallFunction|Attack))))

(event Custom|StopAiming
  ;[1 1 1] AimingEvents
  (Variables|Default|SetbIsAiming false)
  (bind _output_get (Variables|Default|SetCombatState "NewEnumerator2"))
  (AI|Components|Blackboard|SetValueasEnum (AI|GetBlackboard 0) (Utilities|Name|MakeLiteralName "CombatState") _output_get))

(event Custom|StartAiming
  ;[1 1 1] AimingEvents
  (Variables|Default|SetbIsAiming true)
  (bind _output_get (Variables|Default|SetCombatState "NewEnumerator0"))
  (AI|Components|Blackboard|SetValueasEnum (AI|GetBlackboard 0) (Utilities|Name|MakeLiteralName "CombatState") _output_get))

(event Custom|StartAttack
  ;[1 1 1] Shooting
  (CallFunction|Attack))

(event EventBeginPlay
  ;[1 1 1] BeginPlay
  (|CallParentFunction)
  (Utilities|FlowControl|Sequence
    (:then_0
      (bind _asaic_ranged_ai (Utilities|Casting|CastToAIC_RangedAI (Pawn|GetController)))
      (Variables|Default|SetAIController _asaic_ranged_ai))
    (:then_2
      (AI|Components|Blackboard|SetValueasBool (AI|GetBlackboard 0) (Variables|AIBehaviour|Blackboard|GetShouldUseEQSBBKey) (Variables|AIBehaviour|GetbShouldUseEQS)))))

(event EventOnDeathEvent
  ;[1 1 1] On Death Event
  (|CallParentFunction)
  (Utilities|FlowControl|Sequence
    (:then_0
      (bind _leftweapon (Variables|Default|GetLeftWeapon)
        (:then
          (Actor|DestroyActor _leftweapon))
        (:else)))
    (:then_1
      (bind _rightweapon (Variables|Default|GetRightWeapon)
        (:then
          (Actor|DestroyActor _rightweapon))
        (:else)))))

(fn ConstructionScript
  (|CallParentFunction))