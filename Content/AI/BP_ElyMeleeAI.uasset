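; BP_ElyMeleeAI is a melee AI Blueprint that dual-wields weapons, extending a parent that provides the melee attack events.
; On BeginPlay it spawns two actors of WeaponClass, owned and instigated by itself, and snaps them to the right and left melee weapon socket components.
; StartMeleeAttack and EndMeleeAttack call the parent, then forward the start or end attack event to both weapons.
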(event EventBeginPlay
  (bind _self self)
  (bind _self_2 self)
  ;[1 1 1] SpawnWeapons
  (|CallParentFunction)
  (bind _returnvalue (Game|SpawnActorfromClass (Variables|Default|GetWeaponClass) (Transformation|GetActorTransform) "AlwaysSpawn" _self_2 _self_2))
  (Transformation|AttachComponentToComponent _returnvalue (Variables|Default|GetMeleeweaponRightSocket) "" "SnapToTarget" "SnapToTarget" "KeepRelative" true)
  (Variables|Default|SetWeapon%201 _returnvalue)
  (bind _returnvalue_2 (Game|SpawnActorfromClass (Variables|Default|GetWeaponClass) (Transformation|GetActorTransform) "AlwaysSpawn" _self _self))
  (Transformation|AttachComponentToComponent _returnvalue_2 (Variables|Default|GetMeleeweaponLeftSocket) "" "SnapToTarget" "SnapToTarget" "KeepRelative" true)
  (Variables|Default|SetWeapon%202 _returnvalue_2))

(event Collision|EventActorBeginOverlap
  (params (OtherActor :type Actor%20Object%20Reference))
  (|CallParentFunction OtherActor) ; This node is disabled and will not be called.\nDrag off pins to build functionality.
)

(event EventTick
  (params (DeltaSeconds :type Float%20%28single-precision%29))
  (|CallParentFunction DeltaSeconds) ; This node is disabled and will not be called.\nDrag off pins to build functionality.
)

(event EventStartMeleeAttack
  ;[1 1 1] melee Attack
  (|CallParentFunction)
  (Default|StartAttackEvent (Variables|Default|GetWeapon%201))
  (Default|StartAttackEvent (Variables|Default|GetWeapon%202)))

(event EventEndMeleeAttack
  ;[1 1 1] melee Attack
  (|CallParentFunction)
  (Default|EndAttackEvent (Variables|Default|GetWeapon%201))
  (Default|EndAttackEvent (Variables|Default|GetWeapon%202)))

(fn ConstructionScript
  (|CallParentFunction))