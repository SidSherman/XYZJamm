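; Interactable door that loads Level_3_Map once the key-holding enemy is dead.
; On BeginPlay it binds to the death event of the first BP_BaseAI tagged HaveKey, which sets the kill flag.
; A box overlap shows the button prompt and opens a Gate for interaction, which plays a failure sound while the flag is unset.
; Look-at toggles custom depth on the mesh, and telekinesis returns false.
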(event OnComponentBeginOverlap(Box)
  (params (OverlappedComponent :type Primitive%20Component%20Object%20Reference) (OtherActor :type Actor%20Object%20Reference) (OtherComp :type Primitive%20Component%20Object%20Reference) (OtherBodyIndex :type Integer) (bFromSweep :type Boolean) (SweepResult :type Hit%20Result%20Structure%20%28by%20ref%29))
  (Utilities|Casting|CastToBP_PlayerCharacter OtherActor)
  (Rendering|SetVisibility (Variables|Default|GetPressButton_Component) true false)
  (Utilities|FlowControl|Gate false) ; enters at Open
)

(event OnComponentEndOverlap(Box)
  (params (OverlappedComponent :type Primitive%20Component%20Object%20Reference) (OtherActor :type Actor%20Object%20Reference) (OtherComp :type Primitive%20Component%20Object%20Reference) (OtherBodyIndex :type Integer))
  (Utilities|Casting|CastToBP_PlayerCharacter OtherActor)
  (Rendering|SetVisibility (Variables|Default|GetPressButton_Component) false false)
  (Utilities|FlowControl|Gate false) ; enters at Close
)

(event Custom|GetKey
  (Variables|Default|SetEnemyIsKilled? true))

(event EventInteractwith
  (Utilities|FlowControl|Gate false
    (:Exit
      (if (Variables|Default|GetEnemyIsKilled?)
        (Utilities|FlowControl|DoOnce false
          (:Completed
            (Game|OpenLevel(byName) "Level_3_Map")))
        (else
          (Audio|PlaySoundatLocation "/Engine/EditorSounds/Notifications/CompileFailed.CompileFailed" "0, 0, 0" "0, 0, 0" 0.25 1.0 0.0 0 0 0 0))))))

(event EventBeginPlay
  (bind _outactors (Actor|GetAllActorswithTag "HaveKey"))
  (bind _asbp_base_ai (Utilities|Casting|CastToBP_BaseAI (Utilities|Array|Get(acopy) _outactors)))
  (EventDispatchers|BindEventtoOnDeath _asbp_base_ai (delegate Custom|GetKey)))

(fn ConstructionScript)

(fn OnTelekinesis
  (params (HitComponent :type Primitive%20Component%20Object%20Reference))
  (return false))

(fn PlayerLookat
  (params (HitComponent :type Primitive%20Component%20Object%20Reference) (LookAt? :type Boolean))
  (bind _staticmesh (Variables|Default|GetStaticMesh))
  (Rendering|SetRenderCustomDepth _staticmesh LookAt?)
  (return self _staticmesh))