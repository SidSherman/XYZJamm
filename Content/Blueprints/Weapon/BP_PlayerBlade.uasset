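; Melee blade weapon for the player character, used as a left and right pair in which the left blade forwards attack start and end to the right.
; Attacks enable query-only capsule collision and collect unique overlapped actors, then apply damage to all of them shortly after the attack ends.
; Damage comes from the player's blade stat and is scaled by the heavy attack event, while hits during attacks spawn an impact effect.
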(event OnComponentBeginOverlap(Capsule)
  (params (OverlappedComponent :type Primitive%20Component%20Object%20Reference) (OtherActor :type Actor%20Object%20Reference) (OtherComp :type Primitive%20Component%20Object%20Reference) (OtherBodyIndex :type Integer) (bFromSweep :type Boolean) (SweepResult :type Hit%20Result%20Structure%20%28by%20ref%29))
  (if (Math|Boolean|ANDBoolean (!= OtherActor (Game|GetInstigator)) (Variables|Default|GetisAttacking) (!= (Utilities|GetClass OtherActor) "BP_PlayerBlade_C"))
    (Variables|Default|SetHitActor OtherActor)
    (Utilities|Array|AddUnique (Variables|Default|GetHitActorArray) (Variables|Default|GetHitActor))))

(event Custom|HeavyAttack
  (params (Attack :type Boolean))
  (if Attack
    (Variables|Default|SetBase%20Damage (* (Variables|Default|GetBase%20Damage) 1.5))
    (else
      (Variables|Default|SetBase%20Damage (/ (Variables|Default|GetBase%20Damage) 1.5)))))

(event EventBeginPlay
  (bind _returnvalue (Components|GetOwner))
  (Collision|IgnoreActorwhenMoving (Variables|Default|GetCapsule) _returnvalue true)
  (bind _asbp_player_character (Utilities|Casting|CastToBP_PlayerCharacter _returnvalue))
  (bind _output_get (Variables|Default|SetPlayerRef _asbp_player_character))
  (Variables|Default|SetBase%20Damage (Variables|/Game/Characters/Player/BP_PlayerCharacter.BP_PlayerCharacter_C|GetBladeDamage _output_get))
  (EventDispatchers|BindEventtoOnHeavyAttack _asbp_player_character (delegate Custom|HeavyAttack))
  (if (== (Variables|/Game/Characters/Player/BP_PlayerCharacter.BP_PlayerCharacter_C|GetLeftBladeRef (Variables|Default|GetPlayerRef)) self)
    (bind _output_get_2 (Variables|Default|SetDualWeapon (Variables|/Game/Characters/Player/BP_PlayerCharacter.BP_PlayerCharacter_C|GetRightBladeRef (Variables|Default|GetPlayerRef))))
    (Collision|IgnoreActorwhenMoving (Variables|Default|GetCapsule) _output_get_2 true)
    (elif (== (Variables|/Game/Characters/Player/BP_PlayerCharacter.BP_PlayerCharacter_C|GetRightBladeRef (Variables|Default|GetPlayerRef)) self)
      (bind _output_get_3 (Variables|Default|SetPrimaryWeapon (Variables|/Game/Characters/Player/BP_PlayerCharacter.BP_PlayerCharacter_C|GetLeftBladeRef (Variables|Default|GetPlayerRef))))
      (Collision|IgnoreActorwhenMoving (Variables|Default|GetCapsule) _output_get_3 true))))

(event EventEndAttackEvent
  (bind _hitactorarray (Variables|Default|GetHitActorArray))
  (Utilities|FlowControl|Delay 0.2)
  (Variables|Default|SetisAttacking false)
  (Collision|SetCollisionEnabled (Variables|Default|GetCapsule) "NoCollision")
  (bind _dualweapon (Variables|Default|GetDualWeapon)
    (:then
      (Default|EndAttackEvent _dualweapon))
    (:else
      _))
  (for _array_element _hitactorarray
    (CallFunction|DamageEvent :DamagedActor _array_element :Damage (Variables|Default|GetBase%20Damage)))
  (Utilities|Array|Clear _hitactorarray))

(event Collision|EventHit
  (params (MyComp :type Primitive%20Component%20Object%20Reference) (Other :type Actor%20Object%20Reference) (OtherComp :type Primitive%20Component%20Object%20Reference) (bSelfMoved :type Boolean) (HitLocation :type Vector :default "0, 0, 0") (HitNormal :type Vector :default "0, 0, 0") (NormalImpulse :type Vector :default "0, 0, 0") (Hit :type Hit%20Result%20Structure%20%28by%20ref%29))
  (if (Math|Boolean|ANDBoolean (!= Other (Game|GetInstigator)) (Variables|Default|GetisAttacking) (!= Other (Variables|Default|GetDualWeapon)))
    (Effects|SpawnEmitteratLocation "/Game/FX/Particles/Abilities/BladeSiphon/FX/p_Countess_BladeSiphon_HitFX.p_Countess_BladeSiphon_HitFX" HitLocation)))

(event EventDamageEvent
  (params (HitInfo :type Hit%20Result%20Structure) (DamagedActor :type Actor%20Object%20Reference) (Damage :type Float%20%28double-precision%29))
  (Game|Damage|ApplyDamage DamagedActor Damage (Game|GetInstigatorController) (Components|GetOwner)))

(event EventStartAttackEvent
  (Variables|Default|SetisAttacking true)
  (Collision|SetCollisionEnabled (Variables|Default|GetCapsule) "QueryOnly")
  (bind _dualweapon (Variables|Default|GetDualWeapon)
    (:then
      (Default|StartAttackEvent _dualweapon))
    (:else)))

(fn ConstructionScript
  (|CallParentFunction))