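; Player bow weapon that fires arrow projectiles toward the camera's aim point and applies the player's bow damage.
; A camera sphere trace, run every tick and on attack, orients arrows from the arrow mesh to the impact point.
; Attack events gate one spawn per shot and toggle the held arrow, while the damage event adds point damage and a radial impulse.
; The bow swaps to an invisible material through the player's invisibility event.
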(event Custom|SetInvisibilityMod
  (params (isInvisible :type Boolean))
  ;[1 1 1] set player ref
  (Rendering|Material|SetMaterial (Variables|Default|GetStaticMesh) 0 (select isInvisible (stale EventBeginPlay _output_get_2) "/Game/FX/Materials/Heroes/Sparrow/Skins/Rogue/M_Bow_Flames_Inst.M_Bow_Flames_Inst")))

(event EventBeginPlay
  ;[1 1 1] set player ref
  (bind _asbp_player_character (Utilities|Casting|CastToBP_PlayerCharacter (Game|Player|GetPlayerPawn 0)))
  (bind _output_get (Variables|Default|SetPlayerRef _asbp_player_character))
  (bind _returnvalue (Rendering|Material|CreateDynamicMaterialInstance (Variables|Default|GetStaticMesh) 0 "/Game/Material/MI_Inviz.MI_Inviz" "None" :!class /Script/Engine.PrimitiveComponent))
  (bind _output_get_2 (Variables|Default|SetInvisMaterial _returnvalue))
  (EventDispatchers|BindEventtoInvisibility _output_get (delegate Custom|SetInvisibilityMod)))

(event EventEndAttackEvent
  ;[1 1 1] Implement Attack event, start in attack montage
  (Development|SetHiddeninGame (Variables|Default|GetArrowMesh) false false)
  (Utilities|FlowControl|DoOnce false) ; enters at Reset
)

(event EventTick
  (params (DeltaSeconds :type Float%20%28single-precision%29))
  ;[1 1 1] TICK
  (CallFunction|CalculateProjectileInfo))

(event EventStartAttackEvent
  ;[1 1 1] Implement Attack event, start in attack montage
  (bind _returnvalue (CallFunction|CalculateProjectileInfo))
  (Utilities|FlowControl|DoOnce false
    (:Completed
      (Game|SpawnActorfromClass "/Game/Blueprints/Weapon/BP_ArrowProjectile.BP_ArrowProjectile_C" _returnvalue "Undefined" self (Variables|Default|GetPlayerRef))
      (Development|SetHiddeninGame (Variables|Default|GetArrowMesh) true false))))

(event EventDamageEvent
  (params (HitInfo :type Hit%20Result%20Structure) (DamagedActor :type Actor%20Object%20Reference) (Damage :type Float%20%28double-precision%29))
  (bind _playerref (Variables|Default|GetPlayerRef))
  ;[1 1 1] Damage event
  (bind _output_get (Variables|Default|SetHitInfo HitInfo))
  (Game|Damage|ApplyPointDamage DamagedActor (Variables|/Game/Characters/Player/BP_PlayerCharacter.BP_PlayerCharacter_C|GetBowDamage _playerref) (Transformation|GetWorldLocation (Variables|Default|GetStaticMesh)) _output_get (Pawn|GetController _playerref) _playerref)
  (Utilities|IsValid (.HitComponent (Collision|BreakHitResult (Variables|Default|GetHitInfo)))
    (:Is%20Valid
      (Physics|AddRadialImpulse (.HitComponent (Collision|BreakHitResult (Variables|Default|GetHitInfo))) (.ImpactPoint (Collision|BreakHitResult (Variables|Default|GetHitInfo))) 1e+02 4e+03 "RIF_Linear" true))))

(fn ConstructionScript
  (|CallParentFunction))

(fn CalculateProjectileInfo
  (bind _returnvalue (Game|GetPlayerCameraManager 0))
  (bind _returnvalue_2 (Transformation|GetActorLocation _returnvalue))
  (bind _returnvalue_3 (Transformation|GetActorForwardVector _returnvalue))
  (bind _returnvalue_4 (* _returnvalue_3 1.5e+04))
  (bind _returnvalue_5 (+ _returnvalue_2 _returnvalue_4))
  (Variables|Default|SetImpact%20PointLocation _returnvalue_5)
  (bind (_outhit _returnvalue_6) (Collision|SphereTraceByChannel _returnvalue_2 _returnvalue_5 5.0 "TraceTypeQuery1" false (Utilities|Array|MakeArray self (Game|Player|GetPlayerPawn 0)) "None"))
  (Variables|Default|SetHitInfo _outhit)
  (if _returnvalue_6
    (Variables|Default|SetImpact%20PointLocation (.ImpactPoint (Collision|BreakHitResult _outhit))))
  (bind _output_get (Variables|Default|SetArrowSpawnLoc (.location (Transformation|GetWorldTransform (Variables|Default|GetArrowMesh)))))
  (bind _output_get_2 (Variables|Default|SetArrowSpawnRotation (Math|Rotator|MakeRotfromX (- (Variables|Default|GetImpact%20PointLocation) (Variables|Default|GetArrowSpawnLoc)))))
  (return (Math|Transform|MakeTransform _output_get _output_get_2 "0.450000,0.450000,0.450000") (.HitActor (Collision|BreakHitResult _outhit))))