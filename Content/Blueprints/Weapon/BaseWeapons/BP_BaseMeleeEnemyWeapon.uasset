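; Base melee weapon for AI enemies that deals damage to characters it hits during an attack.
; StartAttackEvent and EndAttackEvent toggle the DamageCollision between query-only and no collision.
; Overlapping BP_BaseCharacter actors other than the owner are damaged once per swing, tracked in AttackedActors, which clears when the attack ends.
; Damage is credited to the owner's AI controller, with debug prints on each hit.
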(event OnComponentBeginOverlap(DamageCollision)
  (params (OverlappedComponent :type Primitive%20Component%20Object%20Reference) (OtherActor :type Actor%20Object%20Reference) (OtherComp :type Primitive%20Component%20Object%20Reference) (OtherBodyIndex :type Integer) (bFromSweep :type Boolean) (SweepResult :type Hit%20Result%20Structure%20%28by%20ref%29))
  (bind _attackedactors (Variables|Default|GetAttackedActors))
  ;[1 1 1] ApplyDamage
  (bind _asbp_base_character (Utilities|Casting|CastToBP_BaseCharacter OtherActor))
  (if (!= OtherActor (Components|GetOwner))
    (if (== (Utilities|Array|FindItem _attackedactors _asbp_base_character) -1)
      (Utilities|Array|Add _attackedactors _asbp_base_character)
      (Game|Damage|ApplyDamage _asbp_base_character (Variables|Default|GetDamage) (AI|GetAIController (Components|GetOwner)) self)
      (Development|PrintString "Apply Damage")
      (Development|PrintString (Utilities|GetDisplayName self)))))

(event EventBeginPlay)

(event Collision|EventActorBeginOverlap
  (params (OtherActor :type Actor%20Object%20Reference)))

(event EventTick
  (params (DeltaSeconds :type Float%20%28single-precision%29)))

(event EventStartAttackEvent
  ;[1 1 1] Attack Events
  (Collision|SetCollisionEnabled (Variables|Default|GetDamageCollision) "QueryOnly"))

(event EventEndAttackEvent
  ;[1 1 1] Attack Events
  (Collision|SetCollisionEnabled (Variables|Default|GetDamageCollision) "NoCollision")
  (Utilities|Array|Clear (Variables|Default|GetAttackedActors)))

(fn ConstructionScript
  (|CallParentFunction))