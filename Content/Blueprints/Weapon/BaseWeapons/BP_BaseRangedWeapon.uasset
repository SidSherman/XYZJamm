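; Base ranged weapon Blueprint that fires projectiles for an owning BP_BaseAI.
; Shoot plays muzzle flash and sound, then aims a BP_EnemyProjectile at the blackboard TargetActor with random spread.
; Without a target, it spawns the configurable ProjectileClass along the muzzle's forward direction.
; EndAttackEvent clears the shoot timer, but StartAttackEvent only checks validity, as its timer setup is disconnected.
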(event Custom|Shoot
  (bind _skeletalmesh (Variables|Default|GetSkeletalMesh))
  (bind _spreading (Variables|Default|GetSpreading))
  (bind _spreading_2 (Variables|Default|GetSpreading))
  (bind _spreading_3 (Variables|Default|GetSpreading))
  (bind _spreading_4 (Variables|Default|GetSpreading))
  (bind _returnvalue (Transformation|GetSocketLocation _skeletalmesh "Muzzle"))
  (bind _returnvalue_2 (Transformation|GetSocketRotation _skeletalmesh "Muzzle"))
  (bind _returnvalue_3 (* _spreading_4 -1.0))
  (bind _returnvalue_4 (* _spreading_2 -1.0))
  (bind _returnvalue_5 (Math|Random|RandomFloatinRange _returnvalue_3 _spreading))
  (bind _returnvalue_6 (Math|Random|RandomFloatinRange _returnvalue_4 _spreading_3))
  ;[1 1 1] Shoot
  (Utilities|IsValid self
    (:Is%20Valid
      (Effects|SpawnEmitteratLocation (Variables|Default|GetMuzzleFlash) _returnvalue _returnvalue_2)
      (Audio|PlaySoundatLocation (Variables|Sounds|GetShotSound) _returnvalue "0, 0, 0" 1.0 1.0 0.0 0 0 0 0)
      (bind _asbp_base_ai (Utilities|Casting|CastToBP_BaseAI (Components|GetOwner)))
      (Utilities|IsValid (AI|Components|Blackboard|GetValueasObject (AI|GetBlackboard _asbp_base_ai) (Utilities|Name|MakeLiteralName "TargetActor"))
        (:Is%20Valid
          (bind _asactor (Utilities|Casting|CastToActor (AI|Components|Blackboard|GetValueasObject (AI|GetBlackboard _asbp_base_ai) (Utilities|Name|MakeLiteralName "TargetActor"))))
          (bind _output_get (Variables|Default|SetTarget%20Location (Transformation|GetActorLocation _asactor)))
          (Game|SpawnActorfromClass "/Game/Blueprints/Weapon/BP_EnemyProjectile.BP_EnemyProjectile_C" (Math|Transform|MakeTransform _returnvalue (Math|Rotator|FindLookatRotation _returnvalue (+ (+ _output_get "0,0,50.000000") (Math|Vector|MakeVector 0.0 _returnvalue_6 _returnvalue_6)))) "Undefined" self _asbp_base_ai))
        (:Is%20Not%20Valid
          (Game|SpawnActorfromClass (Variables|Default|GetProjectileClass) (Math|Transform|MakeTransform _returnvalue (Math|Rotator|FindLookatRotation _returnvalue (+ (+ (+ _returnvalue (* (Math|Vector|GetForwardVector _returnvalue_2) (Variables|Default|GetShootDistance))) "0,0,50.000000") (Math|Vector|MakeVector 0.0 _returnvalue_5 _returnvalue_5)))) "Undefined" self _asbp_base_ai))))))

(event EventBeginPlay)

(event Collision|EventActorBeginOverlap
  (params (OtherActor :type Actor%20Object%20Reference)))

(event EventEndAttackEvent
  ;[1 1 1] StopEnding
  (Utilities|IsValid self
    (:Is%20Valid
      (Utilities|Time|ClearandInvalidateTimerbyHandle (Variables|Default|GetShootHandle))
      (Variables|Default|SetbIsShooting false))))

(event EventStartAttackEvent
  ;[1 1 1] Start Shooting
  (Utilities|IsValid self))

(event EventTick
  (params (DeltaSeconds :type Float%20%28single-precision%29)))

(fn ConstructionScript
  (|CallParentFunction))