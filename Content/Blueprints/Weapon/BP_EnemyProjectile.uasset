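; BP_EnemyProjectile is an enemy ranged-weapon projectile that damages the player character.
; On BeginPlay it starts a self-destruct timer, then copies damage from its owning BP_BaseRangedWeapon and sets move-ignores for itself, instigator and owner.
; Any sphere overlap destroys it, but only BP_PlayerCharacter takes damage, credited to the instigator's controller with the owner as causer.
; If the owner cast fails, damage and ignore setup are skipped.
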(event OnComponentBeginOverlap(Sphere)
  (params (OverlappedComponent :type Primitive%20Component%20Object%20Reference) (OtherActor :type Actor%20Object%20Reference) (OtherComp :type Primitive%20Component%20Object%20Reference) (OtherBodyIndex :type Integer) (bFromSweep :type Boolean) (SweepResult :type Hit%20Result%20Structure%20%28by%20ref%29))
  (bind _asbp_player_character (Utilities|Casting|CastToBP_PlayerCharacter OtherActor)
    (:then
      (Game|Damage|ApplyDamage _asbp_player_character (Variables|Default|GetBase%20Damage) (Pawn|GetController (Variables|Actor|GetInstigator)) (Components|GetOwner)))
    (:CastFailed
      _))
  (Actor|DestroyActor))

(event Custom|Destroy%20Self
  (Utilities|Time|ClearandInvalidateTimerbyHandle (Variables|Default|GetDestroyHandle))
  (Actor|DestroyActor))

(event EventBeginPlay
  (bind _staticmesh (Variables|Default|GetStaticMesh))
  (bind _returnvalue (Utilities|Time|SetTimerbyEvent (delegate Custom|Destroy%20Self) 7.0))
  (Variables|Default|SetDestroyHandle _returnvalue)
  (bind _asbp_base_ranged_weapon (Utilities|Casting|CastToBP_BaseRangedWeapon (Components|GetOwner)))
  (Variables|Default|SetBase%20Damage (Variables|/Game/Blueprints/Weapon/BaseWeapons/BP_BaseEnemyWeapon.BP_BaseEnemyWeapon_C|GetDamage _asbp_base_ranged_weapon))
  (Collision|IgnoreActorwhenMoving (Variables|Default|GetSphere) (Variables|Actor|GetInstigator) true)
  (Collision|IgnoreActorwhenMoving (Variables|Default|GetSphere) self true)
  (Collision|IgnoreActorwhenMoving _staticmesh self true)
  (Collision|IgnoreActorwhenMoving _staticmesh (Components|GetOwner) true))

(fn ConstructionScript)