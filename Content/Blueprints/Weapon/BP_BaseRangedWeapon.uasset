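; Base ranged weapon Blueprint that fires repeatedly on a looping AttackDelay timer between its start and end attack events.
; Each shot plays muzzle effect and sound calls, then, for a BP_BaseAI owner, line-traces toward the blackboard TargetActor, falling back to muzzle forward at ShootDistance.
; Spreading randomly rolls the trace endpoint as a world-space vector.
; Traces are debug-drawn, and their hit results are unused, so no damage is applied here.
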(event Custom|Shoot
  (bind _skeletalmesh (Variables|Default|GetSkeletalMesh))
  (bind _returnvalue (Transformation|GetSocketLocation _skeletalmesh "Muzzle"))
  (bind _returnvalue_2 (Transformation|GetSocketRotation _skeletalmesh "Muzzle"))
  ;[1 1 1] Shoot
  (Effects|SpawnEmitteratLocation 0 _returnvalue _returnvalue_2)
  (Audio|PlaySoundatLocation 0 _returnvalue "0, 0, 0" 1.0 1.0 0.0 0 0 0 0)
  (bind _asbp_base_range_ai (Utilities|Casting|CastToBP_BaseAI (Components|GetOwner)))
  (Utilities|IsValid (AI|Components|Blackboard|GetValueasObject (AI|GetBlackboard _asbp_base_range_ai) (Utilities|Name|MakeLiteralName "TargetActor"))
    (:Is%20Valid
      (bind _asactor (Utilities|Casting|CastToActor (AI|Components|Blackboard|GetValueasObject (AI|GetBlackboard _asbp_base_range_ai) (Utilities|Name|MakeLiteralName "TargetActor")))
        (:then
          (Collision|LineTraceByChannel _returnvalue (Math|Vector|RotateVector (Transformation|GetActorLocation _asactor) (Math|Rotator|MakeRotator (Math|Random|RandomFloatinRange (* (Variables|Default|GetSpreading) -1.0) 0.0) 0.0 0.0)) "TraceTypeQuery1" false 0 "ForDuration" true "(R=1.000000,G=0.000000,B=0.000000,A=1.000000)" "(R=0.000000,G=1.000000,B=0.000000,A=1.000000)" 0.5))
        (:CastFailed
          (Collision|LineTraceByChannel _returnvalue (Math|Vector|RotateVector (+ _returnvalue (* (Math|Vector|GetForwardVector _returnvalue_2) (Variables|Default|GetShootDistance))) (Math|Rotator|MakeRotator (Math|Random|RandomFloatinRange (* (Variables|Default|GetSpreading) -1.0) 0.0) 0.0 0.0)) "TraceTypeQuery1" false 0 "ForDuration" true "(R=1.000000,G=0.000000,B=0.000000,A=1.000000)" "(R=0.000000,G=1.000000,B=0.000000,A=1.000000)" 0.5 :!label _label))))
    (:Is%20Not%20Valid
      (goto _label))))

(event EventBeginPlay)

(event Collision|EventActorBeginOverlap
  (params (OtherActor :type Actor%20Object%20Reference)))

(event EventEndAttackEvent
  ;[1 1 1] StopEnding
  (Development|PrintString "End Weapon Attack")
  (Utilities|Time|ClearandInvalidateTimerbyHandle (Variables|Default|GetShootHandle))
  (Variables|Default|SetbIsShooting false))

(event EventStartAttackEvent
  ;[1 1 1] Start Shooting
  (Development|PrintString "Begin Weapon Attack")
  (bind _returnvalue (Utilities|Time|SetTimerbyEvent (delegate Custom|Shoot) (Variables|Default|GetAttackDelay) true))
  (Variables|Default|SetShootHandle _returnvalue)
  (Variables|Default|SetbIsShooting true))

(event EventTick
  (params (DeltaSeconds :type Float%20%28single-precision%29)))

(fn ConstructionScript
  (|CallParentFunction))