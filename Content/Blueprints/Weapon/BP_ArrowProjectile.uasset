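; BP_ArrowProjectile is an arrow projectile that turns toward its target location on spawn and ignores its owner and instigator when moving.
; On box overlap it stops and, given a valid BP_PlayerBow owner, passes the stored hit and zero damage to the bow's DamageEvent.
; It then sticks to the struck actor without collision, spawns an emitter, and after a delay activates particles, hides and destroys itself.
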(event OnComponentBeginOverlap(Box)
  (params (OverlappedComponent :type Primitive%20Component%20Object%20Reference) (OtherActor :type Actor%20Object%20Reference) (OtherComp :type Primitive%20Component%20Object%20Reference) (OtherBodyIndex :type Integer) (bFromSweep :type Boolean) (SweepResult :type Hit%20Result%20Structure%20%28by%20ref%29))
  (bind _returnvalue (Components|GetOwner))
  (bind _projectilemovement (Variables|Default|GetProjectileMovement))
  (if (!= OtherActor self)
    (Components|Movement|StopMovementImmediately _projectilemovement)
    (Variables|/Script/Engine.ProjectileMovementComponent|SetProjectileGravityScale _projectilemovement 0.0)
    (Utilities|IsValid _returnvalue
      (:Is%20Valid
        (bind _asbp_player_bow (Utilities|Casting|CastToBP_PlayerBow _returnvalue))
        (Default|DamageEvent _asbp_player_bow (Variables|Default|GetHit) OtherActor 0.0)
        (Transformation|AttachActorToActor OtherActor "None" "KeepWorld" "KeepWorld" "KeepWorld" true)
        (Collision|SetCollisionEnabled (Variables|Default|GetBox) "NoCollision")
        (Effects|SpawnEmitteratLocation 0 "0, 0, 0")
        (Utilities|FlowControl|Delay 5.0)
        (Components|Activation|Activate (Variables|Default|GetParticleSystem) true)
        (Utilities|FlowControl|Delay 0.5)
        (Development|SetHiddeninGame (Variables|Default|GetArrowMesh) true false)
        (Utilities|FlowControl|Delay 1.0)
        (Actor|DestroyActor)))))

(event EventBeginPlay
  (bind _arrowmesh (Variables|Default|GetArrowMesh))
  (Collision|IgnoreActorwhenMoving _arrowmesh (Game|GetInstigator) true)
  (Collision|IgnoreActorwhenMoving _arrowmesh (Components|GetOwner) true)
  (Transformation|SetActorRotation (Math|Rotator|FindLookatRotation (Transformation|GetActorLocation) (Variables|Default|GetTargetLocation))))

(event Collision|EventHit
  (params (MyComp :type Primitive%20Component%20Object%20Reference) (Other :type Actor%20Object%20Reference) (OtherComp :type Primitive%20Component%20Object%20Reference) (bSelfMoved :type Boolean) (HitLocation :type Vector :default "0, 0, 0") (HitNormal :type Vector :default "0, 0, 0") (NormalImpulse :type Vector :default "0, 0, 0") (Hit :type Hit%20Result%20Structure%20%28by%20ref%29))
  (Variables|Default|SetHit Hit))

(fn ConstructionScript)