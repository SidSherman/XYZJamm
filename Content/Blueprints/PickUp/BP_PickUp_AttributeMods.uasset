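; Pickup actor that upgrades one player attribute (blades, bow, durability, energy, telekinesis or arrow count) when picked up.
; PickUpItem maps its AttrubuteType to a literal Russian name and passes it to BP_PlayerCharacter's UpdragePlayerAttributes.
; It then triggers the character's attribute-change call and destroys itself.
; PlayerLookAt toggles custom depth rendering on the static mesh and returns the actor and mesh.
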(event EventPickUpItem
  (bind _asbp_player_character (Utilities|Casting|CastToBP_PlayerCharacter (Game|Player|GetPlayerPawn 0)))
  (Default|UpdragePlayerAttributes _asbp_player_character (Utilities|Select :Index (Variables|Default|GetAttrubuteType) :NewEnumerator0 (Utilities|Name|MakeLiteralName "Клинки") :NewEnumerator1 (Utilities|Name|MakeLiteralName "Лук") :NewEnumerator2 (Utilities|Name|MakeLiteralName "Прочность") :NewEnumerator3 (Utilities|Name|MakeLiteralName "Энергия") :NewEnumerator4 (Utilities|Name|MakeLiteralName "Телекинез") :NewEnumerator5 (Utilities|Name|MakeLiteralName "Боезапас")))
  (Default|CallOnChangeAttibute _asbp_player_character)
  (Actor|DestroyActor))

(event EventBeginPlay)

(fn ConstructionScript
  (|CallParentFunction))

(fn PlayerLookat
  (params (HitComponent :type Primitive%20Component%20Object%20Reference) (LookAt? :type Boolean))
  (bind _staticmesh (Variables|Default|GetStaticMesh))
  (Rendering|SetRenderCustomDepth _staticmesh LookAt?)
  (return self _staticmesh))