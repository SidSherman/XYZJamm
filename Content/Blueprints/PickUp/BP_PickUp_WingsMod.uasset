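; BP_PickUp_WingsMod is a wings mod pickup that grants the player the Fly and Dash abilities.
; On pickup it looks up Quest06 in DT_Quests, sends it to the player pawn as a quest message, enables both abilities in CanUseAbilityByName, then destroys itself.
; PlayerLookAt toggles custom depth on the mesh while looked at and returns the actor and mesh.
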(event EventPickUpItem
  (bind _returnvalue (Game|Player|GetPlayerPawn 0))
  (bind _returnvalue_2 (Utilities|GetDataTableRow "/Game/Blueprints/QuestSystem/DT_Quests.DT_Quests" "Quest06")
    (:then
      (Class|BPIInteraction|GiveQuesttoPlayer(Message) _returnvalue _returnvalue_2)
      (bind _asbp_player_character (Utilities|Casting|CastToBP_PlayerCharacter _returnvalue))
      (Utilities|Map|Add (Variables|/Game/Characters/Player/BP_PlayerCharacter.BP_PlayerCharacter_C|GetCanUseAbilityByName _asbp_player_character) "Fly" true)
      (Utilities|Map|Add (Variables|/Game/Characters/Player/BP_PlayerCharacter.BP_PlayerCharacter_C|GetCanUseAbilityByName _asbp_player_character) "Dash" true)
      (Actor|DestroyActor))))

(fn ConstructionScript
  (|CallParentFunction))

(fn PlayerLookat
  (params (HitComponent :type Primitive%20Component%20Object%20Reference) (LookAt? :type Boolean))
  (bind _staticmesh (Variables|Default|GetStaticMesh))
  (Rendering|SetRenderCustomDepth _staticmesh LookAt?)
  (return self _staticmesh))