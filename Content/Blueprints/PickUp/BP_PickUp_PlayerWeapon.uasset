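; Pickup actor that gives the player their weapon along with the Quest01 quest.
; On PickUpItem it sends the DT_Quests row to the player pawn, unlocks the Melee ability on BP_PlayerCharacter, spawns the weapon there and destroys itself.
; PlayerLookAt toggles custom depth on the skeletal mesh while looked at, and overlap handling defers to the parent class.
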(event EventBeginPlay
  (|CallParentFunction) ; This node is disabled and will not be called.\nDrag off pins to build functionality.
)

(event Collision|EventActorBeginOverlap
  (params (OtherActor :type Actor%20Object%20Reference))
  (|CallParentFunction OtherActor))

(event EventTick
  (params (DeltaSeconds :type Float%20%28single-precision%29))
  (|CallParentFunction DeltaSeconds) ; This node is disabled and will not be called.\nDrag off pins to build functionality.
)

(event EventPickUpItem
  (bind _returnvalue (Game|Player|GetPlayerPawn 0))
  (bind _returnvalue_2 (Utilities|GetDataTableRow "/Game/Blueprints/QuestSystem/DT_Quests.DT_Quests" "Quest01")
    (:then
      (Class|BPIInteraction|GiveQuesttoPlayer(Message) _returnvalue _returnvalue_2)
      (bind _asbp_player_character (Utilities|Casting|CastToBP_PlayerCharacter _returnvalue))
      (Utilities|Map|Add (Variables|/Game/Characters/Player/BP_PlayerCharacter.BP_PlayerCharacter_C|GetCanUseAbilityByName _asbp_player_character) "Melee" true)
      (Default|SpawnWeapon _asbp_player_character "NewEnumerator0")
      (Actor|DestroyActor))))

(fn ConstructionScript
  (|CallParentFunction))

(fn PlayerLookat
  (params (HitComponent :type Primitive%20Component%20Object%20Reference) (LookAt? :type Boolean))
  (bind _skeletalmesh (Variables|Default|GetSkeletalMesh))
  (Rendering|SetRenderCustomDepth _skeletalmesh LookAt?)
  (return self _skeletalmesh))