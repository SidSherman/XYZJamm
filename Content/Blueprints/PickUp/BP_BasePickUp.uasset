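; BP_BasePickUp is a base Blueprint for items the player picks up through an interact event.
; A trigger overlap with BP_PlayerCharacter opens and closes a gate, so Interactwith only calls PickUpItem while the player is in range.
; A second trigger shows and hides a press-button widget component.
; PickUpItem is left empty for child Blueprints, while telekinesis and look-at functions are stubs, with telekinesis returning false.
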(event OnComponentBeginOverlap(PickUpTrigger)
  (params (OverlappedComponent :type Primitive%20Component%20Object%20Reference) (OtherActor :type Actor%20Object%20Reference) (OtherComp :type Primitive%20Component%20Object%20Reference) (OtherBodyIndex :type Integer) (bFromSweep :type Boolean) (SweepResult :type Hit%20Result%20Structure%20%28by%20ref%29))
  ;[1 1 1] Interacct event
  (Utilities|Casting|CastToBP_PlayerCharacter OtherActor)
  (Utilities|FlowControl|Gate true) ; enters at Open
)

(event OnComponentEndOverlap(PickUpTrigger)
  (params (OverlappedComponent :type Primitive%20Component%20Object%20Reference) (OtherActor :type Actor%20Object%20Reference) (OtherComp :type Primitive%20Component%20Object%20Reference) (OtherBodyIndex :type Integer))
  ;[1 1 1] Interacct event
  (Utilities|Casting|CastToBP_PlayerCharacter OtherActor)
  (Utilities|FlowControl|Gate true) ; enters at Close
)

(event OnComponentBeginOverlap(WidgetVisibilityTrigger)
  (params (OverlappedComponent :type Primitive%20Component%20Object%20Reference) (OtherActor :type Actor%20Object%20Reference) (OtherComp :type Primitive%20Component%20Object%20Reference) (OtherBodyIndex :type Integer) (bFromSweep :type Boolean) (SweepResult :type Hit%20Result%20Structure%20%28by%20ref%29))
  ;[1 1 1] Set visibility of Widget component
  (Utilities|Casting|CastToBP_PlayerCharacter OtherActor)
  (Rendering|SetVisibility (Variables|Default|GetPressButton_Component) true false))

(event OnComponentEndOverlap(WidgetVisibilityTrigger)
  (params (OverlappedComponent :type Primitive%20Component%20Object%20Reference) (OtherActor :type Actor%20Object%20Reference) (OtherComp :type Primitive%20Component%20Object%20Reference) (OtherBodyIndex :type Integer))
  ;[1 1 1] Set visibility of Widget component
  (Utilities|Casting|CastToBP_PlayerCharacter OtherActor)
  (Rendering|SetVisibility (Variables|Default|GetPressButton_Component) false false))

(event Custom|PickUpItem
  ;[1 1 1] Set visibility of Widget component
  ;;[1 1 1] this event must be implementing in child BP
)

(event EventInteractwith
  ;[1 1 1] Interacct event
  (Utilities|FlowControl|Gate true
    (:Exit
      (CallFunction|PickUpItem))))

(fn ConstructionScript)

(fn OnTelekinesis
  (params (HitComponent :type Primitive%20Component%20Object%20Reference))
  (return false))

(fn PlayerLookat
  (params (HitComponent :type Primitive%20Component%20Object%20Reference) (LookAt? :type Boolean))
  (return 0 0))