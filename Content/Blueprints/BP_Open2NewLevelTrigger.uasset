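; BP_Open2NewLevelTrigger is an interactable control panel that moves the player on to Level_2_Map.
; Overlapping its box shows a press-button prompt and opens a gate, so Interactwith only works while the player is in range.
; A single-fire interact flags the player, copies PlayerModifications into the existing SaveGame slot, saves, then opens the level.
; PlayerLookAt highlights the panel through custom depth, and telekinesis always returns false.
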(event OnComponentBeginOverlap(Box)
  (params (OverlappedComponent :type Primitive%20Component%20Object%20Reference) (OtherActor :type Actor%20Object%20Reference) (OtherComp :type Primitive%20Component%20Object%20Reference) (OtherBodyIndex :type Integer) (bFromSweep :type Boolean) (SweepResult :type Hit%20Result%20Structure%20%28by%20ref%29))
  (bind _asbp_player_character (Utilities|Casting|CastToBP_PlayerCharacter OtherActor))
  (Rendering|SetVisibility (Variables|Default|GetPressButton_Component) true false)
  (Utilities|FlowControl|Gate false) ; enters at Open
)

(event OnComponentEndOverlap(Box)
  (params (OverlappedComponent :type Primitive%20Component%20Object%20Reference) (OtherActor :type Actor%20Object%20Reference) (OtherComp :type Primitive%20Component%20Object%20Reference) (OtherBodyIndex :type Integer))
  (Utilities|Casting|CastToBP_PlayerCharacter OtherActor)
  (Rendering|SetVisibility (Variables|Default|GetPressButton_Component) false false)
  (Utilities|FlowControl|Gate false) ; enters at Close
)

(event EventInteractwith
  (Utilities|FlowControl|Gate false
    (:Exit
      (Utilities|FlowControl|DoOnce false
        (:Completed
          (Variables|/Game/Characters/Player/BP_PlayerCharacter.BP_PlayerCharacter_C|SetToNewLevelDestroed (stale OnComponentBeginOverlap(Box) _asbp_player_character) true)
          (bind _returnvalue (SaveGame|LoadGamefromSlot "SaveGame"))
          (bind _asbp_save_game (Utilities|Casting|CastToBP_SaveGame _returnvalue))
          (Variables|/Game/Blueprints/Core/BP_SaveGame.BP_SaveGame_C|SetPlayerAttributes _asbp_save_game (Variables|/Game/Characters/Player/BP_PlayerCharacter.BP_PlayerCharacter_C|GetPlayerModifications (stale OnComponentBeginOverlap(Box) _asbp_player_character)))
          (SaveGame|SaveGametoSlot _asbp_save_game "SaveGame")
          (Game|OpenLevel(byName) "Level_2_Map"))))))

(fn ConstructionScript)

(fn OnTelekinesis
  (params (HitComponent :type Primitive%20Component%20Object%20Reference))
  (return false))

(fn PlayerLookat
  (params (HitComponent :type Primitive%20Component%20Object%20Reference) (LookAt? :type Boolean))
  (bind _sm_controlpanel (Variables|Default|GetSM_ControlPanel))
  (Rendering|SetRenderCustomDepth _sm_controlpanel LookAt?)
  (return self _sm_controlpanel))