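; Trigger volume that hands the player a quest, once, when they enter its box while on the prerequisite quest.
; On BeginPlay it loads its quest row from DT_Quests by name, printing an on-screen error if missing.
; On overlap it looks up the previous quest's row, compares its QuestText to the player's current quest, then calls GiveQuestToPlayerMessage.
; Telekinesis and look-at functions are empty stubs.
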(event OnComponentBeginOverlap(Box)
  (params (OverlappedComponent :type Primitive%20Component%20Object%20Reference) (OtherActor :type Actor%20Object%20Reference) (OtherComp :type Primitive%20Component%20Object%20Reference) (OtherBodyIndex :type Integer) (bFromSweep :type Boolean) (SweepResult :type Hit%20Result%20Structure%20%28by%20ref%29))
  (bind _asbp_player_character (Utilities|Casting|CastToBP_PlayerCharacter OtherActor))
  (bind _returnvalue (Utilities|GetDataTableRow "/Game/Blueprints/QuestSystem/DT_Quests.DT_Quests" (Utilities|Struct|BreakS_Quest (Variables|Default|GetQuest)))
    (:then
      (if (Utilities|Enum|Equal(Enum) (.questtext _returnvalue) (.questtext (Variables|/Game/Characters/Player/BP_PlayerCharacter.BP_PlayerCharacter_C|GetCurrentQuest _asbp_player_character)))
        (Utilities|FlowControl|DoOnce false
          (:Completed
            (Class|BPIInteraction|GiveQuesttoPlayer(Message) _asbp_player_character (Variables|Default|GetQuest))))))))

(event EventBeginPlay
  (bind _returnvalue (Utilities|GetDataTableRow "/Game/Blueprints/QuestSystem/DT_Quests.DT_Quests" (Variables|Default|GetQuestRowName))
    (:then
      (Variables|Default|SetQuest _returnvalue))
    (:RowNotFound
      (Development|PrintText (Utilities|Text|FormatText (Utilities|GetDisplayName self) "{self} can find Quest Row Name in Data table") true true "(R=1.000000,G=0.015401,B=0.000000,A=1.000000)" 1e+01))))

(fn ConstructionScript)

(fn OnTelekinesis
  (params (HitComponent :type Primitive%20Component%20Object%20Reference))
  (return false))

(fn PlayerLookat
  (params (HitComponent :type Primitive%20Component%20Object%20Reference) (LookAt? :type Boolean))
  (return 0 0))