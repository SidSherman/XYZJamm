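; BP_TrainingDoll is a hittable training dummy that gives the player a quest.
; At BeginPlay it loads the Quest02 row from DT_Quests.
; Each hit from BP_PlayerCharacter plays a sound and raises a counter; once it reaches ten, a DoOnce sends that quest to the player.
; It toggles custom depth on its mesh when looked at and returns false for telekinesis.
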(event EventBeginPlay
  (|CallParentFunction)
  (bind _returnvalue (Utilities|GetDataTableRow "/Game/Blueprints/QuestSystem/DT_Quests.DT_Quests" "Quest02")))

(event Game|Damage|EventAnyDamage
  (params (Damage :type Float%20%28single-precision%29) (DamageType :type Damage%20Type%20Object%20Reference) (InstigatedBy :type Controller%20Object%20Reference) (DamageCauser :type Actor%20Object%20Reference))
  (bind _hitcount (Variables|Default|GetHitCount))
  (bind _asbp_player_character (Utilities|Casting|CastToBP_PlayerCharacter DamageCauser))
  (Audio|PlaySound2D "/Game/Sound/Footstep/Cue/SCue_Glass_Footstep.SCue_Glass_Footstep" 1.0 1.0 0.0 0 0)
  (Math|Integer|IncrementInt _hitcount
    (:%20%20
      (if (>= _hitcount 10)
        (Utilities|FlowControl|DoOnce false
          (:Completed
            (Class|BPIInteraction|GiveQuesttoPlayer(Message) _asbp_player_character (stale EventBeginPlay _returnvalue))))))))

(fn ConstructionScript
  (|CallParentFunction))

(fn OnTelekinesis
  (params (HitComponent :type Primitive%20Component%20Object%20Reference))
  (return false))

(fn PlayerLookat
  (params (HitComponent :type Primitive%20Component%20Object%20Reference) (LookAt? :type Boolean))
  (Rendering|SetRenderCustomDepth (Variables|Character|GetMesh) LookAt?)
  (return self (Variables|Character|GetMesh)))