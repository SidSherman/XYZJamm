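; BP_MainMenuPanel is an in-world main menu with start and exit options built from text renders and clickable boxes.
; Cursor-over events on each box switch its text between the base and active colors.
; Start loads the "SaveGame" slot and opens its saved level, or Map_Start when that name is None; a failed save cast opens nothing.
; Exit quits the game.
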(event OnBeginCursorOver(StartGameBox)
  (params (TouchedComponent :type Primitive%20Component%20Object%20Reference))
  (Rendering|Components|TextRender|SetTextRenderColor (Variables|Default|GetStartGameText) (Variables|Default|GetActiveStringColor)))

(event OnEndCursorOver(StartGameBox)
  (params (TouchedComponent :type Primitive%20Component%20Object%20Reference))
  (Rendering|Components|TextRender|SetTextRenderColor (Variables|Default|GetStartGameText) (Variables|Default|GetBaseStringColor)))

(event OnBeginCursorOver(ExitGameBox)
  (params (TouchedComponent :type Primitive%20Component%20Object%20Reference))
  (Rendering|Components|TextRender|SetTextRenderColor (Variables|Default|GetExitGame) (Variables|Default|GetActiveStringColor)))

(event OnEndCursorOver(ExitGameBox)
  (params (TouchedComponent :type Primitive%20Component%20Object%20Reference))
  (Rendering|Components|TextRender|SetTextRenderColor (Variables|Default|GetExitGame) (Variables|Default|GetBaseStringColor)))

(event OnClicked(StartGameBox)
  (params (TouchedComponent :type Primitive%20Component%20Object%20Reference) (ButtonPressed :type Key%20Structure :default "None"))
  (bind _returnvalue (SaveGame|LoadGamefromSlot "SaveGame"))
  (bind _asbp_save_game (Utilities|Casting|CastToBP_SaveGame _returnvalue))
  (if (!= (Variables|/Game/Blueprints/Core/BP_SaveGame.BP_SaveGame_C|GetCurrentLevelName _asbp_save_game) "")
    (Game|OpenLevel(byName) (Variables|/Game/Blueprints/Core/BP_SaveGame.BP_SaveGame_C|GetCurrentLevelName _asbp_save_game))
    (else
      (Game|OpenLevel(byName) "Map_Start"))))

(event OnClicked(ExitGameBox)
  (params (TouchedComponent :type Primitive%20Component%20Object%20Reference) (ButtonPressed :type Key%20Structure :default "None"))
  (Game|QuitGame 0 "Quit" false))

(event EventBeginPlay)

(fn ConstructionScript)