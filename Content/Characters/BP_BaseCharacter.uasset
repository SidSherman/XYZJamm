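; BP_BaseCharacter is a base character Blueprint that provides health, damage and death handling.
; AnyDamage ignores damage whose InstigatedBy equals self and passes the rest as a negative value to ModifyCurrentHeath.
; That function caps health at MaxHealth and, when health drops to zero or below, runs OnDeathEvent, which calls OnDeath.
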(event Custom|OnDeathEvent
  (Default|CallOnDeath))

(event EventBeginPlay)

(event Collision|EventActorBeginOverlap
  (params (OtherActor :type Actor%20Object%20Reference)))

(event EventTick
  (params (DeltaSeconds :type Float%20%28single-precision%29)))

(event Game|Damage|EventAnyDamage
  (params (Damage :type Float%20%28single-precision%29) (DamageType :type Damage%20Type%20Object%20Reference) (InstigatedBy :type Controller%20Object%20Reference) (DamageCauser :type Actor%20Object%20Reference))
  (if (!= InstigatedBy self)
    (CallFunction|ModifyCurrentHeath (* Damage -1.0))))

(fn ConstructionScript)

(fn ModifyCurrentHeath
  (params (Value :type Float%20%28double-precision%29))
  (if (>= (+ (Variables|Default|GetCurrentHealth) Value) (Variables|Attribute|GetMaxHealth))
    (Variables|Default|SetCurrentHealth (Variables|Attribute|GetMaxHealth))
    (else
      (bind _output_get (Variables|Default|SetCurrentHealth (+ (Variables|Default|GetCurrentHealth) Value)))
      (if (<= _output_get 0.0)
        (CallFunction|OnDeathEvent)))))