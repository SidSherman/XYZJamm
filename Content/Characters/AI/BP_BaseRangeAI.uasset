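; Base ranged enemy AI character that spawns a weapon into its hand socket and feeds player perception into its Blackboard.
; Sighting the player sets the target and starts a caution timer that switches state to Agressive, immediately if within range.
; Losing sight saves the target's last position and clears it.
; Noise stimuli write a heard location, but only while a target is set; aiming events are empty stubs.
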(event OnPerceptionUpdated(AIPerception)
  (params (UpdatedActors :type Array%20of%20Actor%20Object%20References))
  (bind _returnvalue (AI|GetBlackboard 0))
  (bind _returnvalue_2 (AI|GetBlackboard 0))
  (bind _out (CallFunction|GetCharfrom UpdatedActors))
  (bind _returnvalue_3 (AI|GetBlackboard 0))
  (bind _returnvalue_4 (AI|GetBlackboard 0))
  ;[0.1521 0.477 1] Sight Reciver
  ;;[1 1 1] FindPlayerCharacter
  (Utilities|IsValid _out
    (:Is%20Valid
      (if (!= (Utilities|Array|FindItem (Class|AIPerceptionComponent|GetCurrentlyPerceivedActors (Variables|Default|GetAIPerception) "/Script/AIModule.AISense_Sight") _out) -1)
        (bind _output_get (Variables|AIBehaviour|SetTargetActor _out))
        ;;[1 1 1] Set Target
        (Utilities|IsValid _returnvalue_3
          (:Is%20Valid
            (AI|Components|Blackboard|SetValueasObject _returnvalue_3 (Variables|AIBehaviour|GetTargetActorBBKey) _output_get)
            (AI|Components|Blackboard|SetValueasBool _returnvalue_3 (Variables|AIBehaviour|GetHasLostTimerBBKey) false)
            ;;;[1 1 1] Time To SetArressiveState
            (bind _returnvalue_5 (Utilities|Time|SetTimerbyEvent (delegate Custom|CatiousTimer) (Variables|AIBehaviour|GetCatiousTime)))
            (Variables|AIBehaviour|SetCatiousTimerHandle _returnvalue_5)
            (Utilities|IsValid (Variables|AIBehaviour|GetTargetActor)
              (:Is%20Valid
                (if (<= (Math|Vector|Distance(Vector) (Transformation|GetActorLocation (Variables|AIBehaviour|GetTargetActor)) (Transformation|GetActorLocation)) (Variables|AIBehaviour|GetAgressiveDistance))
                  (CallFunction|CatiousTimer))))))
        (else
          ;;[1 1 1] Forget About Target
          (if (Utilities|Enum|Equal(Enum) (Variables|AIBehaviour|GetAIState) "NewEnumerator0")
            (bind _output_get_2 (Variables|AIBehaviour|SetAIState "NewEnumerator0")))
          (Utilities|IsValid _returnvalue_2
            (:Is%20Valid
              (AI|Components|Blackboard|SetValueasEnum _returnvalue_2 (Variables|AIBehaviour|GetAIStateBBKey) _output_get_2)
              (AI|Components|Blackboard|SetValueasBool _returnvalue (Variables|AIBehaviour|GetHasLostTimerBBKey) true)
              (bind _asactor (Utilities|Casting|CastToActor (AI|Components|Blackboard|GetValueasObject _returnvalue (Variables|AIBehaviour|GetTargetActorBBKey))))
              (AI|Components|Blackboard|SetValueasVector _returnvalue_4 (Utilities|Name|MakeLiteralName "TargetPosition") (Transformation|GetActorLocation _asactor))
              (AI|Components|Blackboard|ClearValue _returnvalue_4 (Variables|AIBehaviour|GetTargetActorBBKey)))))))))

(event OnTargetPerceptionUpdated(AIPerception)
  (params (Actor :type Actor%20Object%20Reference) (Stimulus :type AI%20Stimulus%20Structure))
  ;[1 0.8899 0.1083] Hearing Reciever
  (if (== (.tag Stimulus) "Noise")
    (Utilities|IsValid (AI|Components|Blackboard|GetValueasObject (AI|GetBlackboard 0) (Variables|AIBehaviour|GetTargetActorBBKey))
      (:Is%20Valid
        (Utilities|Casting|CastToBP_PlayerCharacter Actor)
        (Development|PrintString "AI Heard Player" true true "(R=0.000000,G=0.660000,B=1.000000,A=1.000000)" 2.0 "2")
        (AI|Components|Blackboard|SetValueasBool (AI|GetBlackboard 0) (Variables|AIBehaviour|GetTargetPositionUpdatedBBKey) true)
        (switch Utilities|FlowControl|Switch|SwitchonEAIStates (Variables|AIBehaviour|GetAIState)
          (:NewEnumerator0
            (bind _output_get (Variables|AIBehaviour|SetAIState "NewEnumerator0"))
            (AI|Components|Blackboard|SetValueasEnum (AI|GetBlackboard 0) (Variables|AIBehaviour|GetAIStateBBKey) _output_get))
          (:NewEnumerator1
            _)
          (:NewEnumerator2
            _)
          (:NewEnumerator4
            _))
        (AI|Components|Blackboard|SetValueasVector (AI|GetBlackboard 0) (Variables|AIBehaviour|GetTargetPositionBBKey) (.stimuluslocation Stimulus))
        (AI|Components|Blackboard|SetValueasBool (AI|GetBlackboard 0) (Variables|AIBehaviour|GetTargetPositionUpdatedBBKey) true)
        (AI|Components|Blackboard|SetValueasBool (AI|GetBlackboard 0) (Variables|AIBehaviour|GetHeardSometingBBKey) true)))))

(event Custom|CatiousTimer
  ;[0.1521 0.477 1] Sight Reciver
  ;;[1 1 1] Set Target
  ;;;[1 1 1] Time To SetArressiveState
  (AI|Components|Blackboard|ClearValue (AI|GetBlackboard 0) (Variables|AIBehaviour|GetHasLostTimerBBKey))
  (Utilities|Time|ClearandInvalidateTimerbyHandle (Variables|AIBehaviour|GetCatiousTimerHandle))
  (bind _output_get (Variables|AIBehaviour|SetAIState "NewEnumerator2"))
  (AI|Components|Blackboard|SetValueasEnum (AI|GetBlackboard 0) (Variables|AIBehaviour|GetAIStateBBKey) _output_get))

(event Custom|StopAiming
  ;[1 1 1] AimingEvents
)

(event Custom|StartAiming
  ;[1 1 1] AimingEvents
)

(event EventBeginPlay
  (bind _self self)
  ;[1 1 1] BeginPlay
  (|CallParentFunction)
  (bind _asaic_ranged_ai (Utilities|Casting|CastToAIC_RangedAI (Pawn|GetController)))
  (Variables|AIBehaviour|SetAIController _asaic_ranged_ai)
  (bind _returnvalue (Game|SpawnActorfromClass (Variables|Default|GetWeaponClass) (Transformation|GetActorTransform) "AlwaysSpawn" _self _self))
  (Transformation|AttachComponentToComponent _returnvalue (Variables|Character|GetMesh) "WeaponSocket" "SnapToTarget" "SnapToTarget" "KeepRelative" true)
  (Variables|AIBehaviour|SetWeapon _returnvalue))

(event EventTick
  (params (DeltaSeconds :type Float%20%28single-precision%29))
  ;[1 1 1] Debug
)

(fn ConstructionScript
  (|CallParentFunction))

(fn GetCharfrom
  (params (Input :type Array%20of%20Actor%20Object%20References))
  (for _array_element Input
    (bind _asbp_player_character (Utilities|Casting|CastToBP_PlayerCharacter _array_element))
    (return _asbp_player_character)))